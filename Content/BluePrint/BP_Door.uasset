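; BP_Door is a door actor that slides open and closed when its Interaction function is called.
; Interaction toggles the Ouvert flag and calls Ouvrir or Fermer, which play or reverse the OuvertureFermeture timeline.
; The timeline lerps the actor's location, without sweep, from the position saved at BeginPlay to that position plus the PositionOuvert offset.
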(event Custom|Ouvrir
  (bind _positiondepart (Variables|Default|GetPositionDepart))
  (bind _track (Timeline|Ouverture%20Fermeture Play)
    (:Update
      (Transformation|SetActorLocation (Math|Vector|Lerp(Vector) _positiondepart (+ _positiondepart (Variables|Default|GetPositionOuvert)) _track) false false))))

(event Custom|Fermer
  (bind _positiondepart (Variables|Default|GetPositionDepart))
  (bind _track (Timeline|Ouverture%20Fermeture Reverse)
    (:Update
      (Transformation|SetActorLocation (Math|Vector|Lerp(Vector) _positiondepart (+ _positiondepart (Variables|Default|GetPositionOuvert)) _track) false false))))

(event EventBeginPlay
  (Variables|Default|SetPositionDepart (Transformation|GetActorLocation)))

(event Collision|EventActorBeginOverlap
  (params (OtherActor :type Actor%20Object%20Reference)))

(event EventTick
  (params (DeltaSeconds :type Float%20%28single-precision%29)))

(fn ConstructionScript)

(fn Interaction
  (if (Variables|Default|GetOuvert)
    (CallFunction|Fermer)
    (Variables|Default|SetOuvert false)
    (else
      (CallFunction|Ouvrir)
      (Variables|Default|SetOuvert true))))